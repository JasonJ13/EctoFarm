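; BP_Fairy is a fairy actor that wanders by moving its mesh along curving paths.
; Each Tick advances the mesh along its local X while yawing it, with a random chance to reverse the turn direction.
; A Disapear function, not called from this event graph, destroys the actor beyond a set distance from its local origin or at random.
; Destruction also triggers CallQueueFree.
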(event `self.ReceiveTick`
  (params (DeltaSeconds :type "Float (single-precision)"))
  (`self.rotate` DeltaSeconds)
  (`self.change_rotation`))

(event `self.ReceiveDestroyed`
  (`self.QueueFree`))

(fn `change_rotation`
  (locals (ROTATIONCHANCE :type "Float (double-precision)" :default 10.0))
  (if (< (`KismetMathLibrary.RandomInteger` 1000) (`local.ROTATIONCHANCE`))
    (set `self.rotation_dir` (* (`self.rotation_dir`) -1))
    (return)))

(fn `check_distance`
  (returns (pass_distance_max :type Boolean))
  (return (< 300.0 (`KismetMathLibrary.Vector_Distance` (`SceneComponent.RelativeLocation` (`self.SKM_Fairy`))))))

(fn `disapear`
  (bind _pass_distance_max (`self.check_distance`))
  (if (or _pass_distance_max (< (`KismetMathLibrary.RandomInteger` 1000) 1))
    (`self.QueueFree`)
    (`self.K2_DestroyActor`))
  (return))

(fn `rotate`
  (params (delta :type "Float (double-precision)"))
  (locals (ROTATION :type "Float (double-precision)" :default 100.0) (PROGRESS :type "Float (double-precision)" :default 100.0))
  (`SceneComponent.K2_AddLocalRotation` (`self.SKM_Fairy`) (`KismetMathLibrary.MakeRotator` 0.0 0.0 (* delta (`local.ROTATION`) (`self.rotation_dir`))) false false)
  (`SceneComponent.K2_AddLocalOffset` (`self.SKM_Fairy`) (`KismetMathLibrary.MakeVector` (* delta (`local.PROGRESS`))) false false))

(fn `UserConstructionScript`)