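; Fairy spawner that adds a BP_Fairy every two seconds while fewer than 40 are counted.
; Each fairy is a child actor component placed at a random evenly stepped point along one of three fixed relative lines.
; The spawner binds to each fairy's QueueFree event and keeps a live count, with a handler that decrements it and a debug print on every change.
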(event `self.ReceiveBeginPlay`
  (`KismetSystemLibrary.Delay` 2.0 :!label _label)
  (`self.NewFairySpawn`)
  (goto _label))

(event `NewFairySpawn`
  (`self.Fairy_spawn`))

(event `QueueFreeFairy_event`
  (`self.Add_Fairy` -1))

(fn `Add_Fairy`
  (params (nmb_Added :type Integer))
  (bind _output_get (set `self.nmb_Fairy` (+ nmb_Added (`self.nmb_Fairy`))))
  (`KismetSystemLibrary.PrintString` (`KismetStringLibrary.Conv_IntToString` _output_get)))

(fn `Fairy_spawn`
  (if (< (`self.nmb_Fairy`) 40)
    (bind _newparam (`self.Get_Random_Location`))
    ; Add a new fairy with random location
    (bind _returnvalue (`AddComponent|NODE_AddChildActorComponent-2` :`RelativeTransform` (`KismetMathLibrary.MakeTransform` _newparam)))
    ; Set Up Fairy
    (bind _asbp_fairy (cast `/Game/Blueprints/Fairy/BP_Fairy` (`ChildActorComponent.ChildActor` _returnvalue)))
    (add `/Game/Blueprints/Fairy/BP_Fairy.QueueFree` _asbp_fairy (`|CreateDelegate` :!event `QueueFreeFairy_event`))
    (`self.Add_Fairy` 1))
  (return))

(fn `Get_Random_Location`
  (returns (NewParam :type "Vector Structure"))
  (locals (DIVISION :type Integer :default 100) (MAX_DISTANCE :type "Float (double-precision)" :default -3000.0) (OFFSET :type "Float (double-precision)" :default -1000.0))
  (bind _returnvalue (+ (* (`KismetMathLibrary.Conv_IntToDouble` (`KismetMathLibrary.RandomInteger` (`local.DIVISION`))) (/ (`local.MAX_DISTANCE`) (`KismetMathLibrary.Conv_IntToDouble` (`local.DIVISION`)))) (`local.OFFSET`)))
  (switch `int` (`KismetMathLibrary.RandomInteger` 3)
    (:`0`
      (return (`KismetMathLibrary.MakeVector` _returnvalue -1000.0 36.0)))
    (:`1`
      (return (`KismetMathLibrary.MakeVector` _returnvalue -4000.0 36.0)))
    (:`2`
      (return (`KismetMathLibrary.MakeVector` -4000.0 _returnvalue 36.0)))))

(fn `UserConstructionScript`)