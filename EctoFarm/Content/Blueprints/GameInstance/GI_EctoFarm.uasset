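; GI_EctoFarm is the game instance for a farming game, holding the dirtland list and the player's money and score.
; Dirtlands register through NewDirtland, and the Night_Phase event calls Night on each one, passing the disaster and its array index.
; PlantGrow adds a plant's score to the player total, while PlantHarvest adds its money.
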(event `Night_Phase`
  (params (Disaster :type "/Game/Blueprints/Enum/E_Disaster Enum" :default "NewEnumerator0"))
  (for (_array_element _array_index) (`self.dirtlands`)
    (`/Game/Blueprints/Dirtland/BP_Dirtland.Night` _array_element Disaster (`KismetMathLibrary.Conv_IntToDouble` _array_index))))

(fn `New_Dirtland`
  (params (NewParam :type "/Game/Blueprints/Dirtland/BP_Dirtland Object Reference"))
  (`KismetArrayLibrary.Array_Add` (`self.dirtlands`) NewParam))

(fn `Plant_Grow`
  (params (NewParam :type "/Game/Blueprints/Dirtland/Plant/BP_Plant Object Reference"))
  (locals (plante :type "/Game/Blueprints/Dirtland/Plant/BP_Plant Object Reference"))
  (set `local.plante` NewParam)
  (set `self.Score_Player` (+ (`/Game/Blueprints/Dirtland/Plant/BP_Plant.Score` (`local.plante`)) (`self.Score_Player`))))

(fn `Plant_Harvest`
  (params (Plant :type "/Game/Blueprints/Dirtland/Plant/BP_Plant Object Reference"))
  (locals (Plante :type "/Game/Blueprints/Dirtland/Plant/BP_Plant Object Reference"))
  (set `local.Plante` Plant)
  (set `self.Money_Player` (+ (`/Game/Blueprints/Dirtland/Plant/BP_Plant.Money` (`local.Plante`)) (`self.Money_Player`)))
  (return))