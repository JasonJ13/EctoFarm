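; BP_Dirtland is a farm plot actor that holds up to three plants, planting corn on interaction or watering thirsty plants when full.
; Plants reposition to preset offsets as their count changes through planting, harvesting grown ones or random removal.
; A survival check sums plant resistances against a threshold.
; The Visualizer's material shows reachability and selection outlines, with BP_Farmer selection taking priority over BP_Phantom.
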(event `self.ReceiveActorBeginOverlap`
  (params (OtherActor :type "Actor Object Reference")))

(event `self.ReceiveActorEndOverlap`
  (params (OtherActor :type "Actor Object Reference")))

(event `self.ReceiveBeginPlay`
  (`PrimitiveComponent.SetMaterial` (`self.Visualizer`) 0 (`self.DefaultMaterial`)))

(fn `Add_Plant`
  (params (NewPlant :type "/Game/Blueprints/Dirtland/Plant/BP_Plant Class Reference"))
  (locals (List_Position :type "Set of Vector Structure") (New_Plant_Class :type "/Game/Blueprints/Dirtland/Plant/BP_Plant Class Reference"))
  (bind (_returnvalue_location _returnvalue_rotation _returnvalue_scale) (`KismetMathLibrary.BreakTransform` (`self.GetTransform`)))
  (set `local.New_Plant_Class` NewPlant)
  (bind _newparam (`self.Relocate_Plant` true))
  (bind _returnvalue (`|SpawnActorFromClass` (`local.New_Plant_Class`) (`KismetMathLibrary.MakeTransform` (+ _newparam _returnvalue_location) _returnvalue_rotation _returnvalue_scale) "Undefined" "MultiplyWithRoot" null null))
  (`KismetArrayLibrary.Array_Add` (`self.Plants`) _returnvalue)
  (return))

(fn `Erase_All_Plant`
  (locals (Temporary_Plants :type "Array of /Game/Blueprints/Dirtland/Plant/BP_Plant Object Reference"))
  (bind _output_get (set `local.Temporary_Plants` (`self.Plants`)))
  (for _array_element _output_get
    (`KismetArrayLibrary.Array_RemoveItem` (`self.Plants`) _array_element)
    (`self.K2_DestroyActor` _array_element))
  (return))

(fn `Erase_One_Plant`
  (bind _plants (`self.Plants`))
  (bind _outitem (`KismetArrayLibrary.Array_Random` _plants))
  (if (`KismetArrayLibrary.Array_IsEmpty` _plants)
    (return)
    (else
      (`self.K2_DestroyActor` _outitem)
      (`KismetArrayLibrary.Array_RemoveItem` _plants _outitem)
      (`self.Relocate_Plant` false))))

(fn `Harvest`
  (locals (To_Remove :type "Array of /Game/Blueprints/Dirtland/Plant/BP_Plant Object Reference"))
  (for _array_element (`self.Plants`)
    (if (`/Game/Blueprints/Dirtland/Plant/BP_Plant.Grown` _array_element)
      (`KismetArrayLibrary.Array_Add` (`local.To_Remove`) _array_element)))
  (for _array_element_2 (`local.To_Remove`)
    (`self.K2_DestroyActor` _array_element_2)
    (`KismetArrayLibrary.Array_RemoveItem` (`self.Plants`) _array_element_2))
  (`KismetSystemLibrary.PrintString` (`KismetStringLibrary.Conv_IntToString` (`KismetArrayLibrary.Array_Length` (`self.Plants`))))
  (`self.Relocate_Plant` false))

(fn `Interaction`
  (if (< (`KismetArrayLibrary.Array_Length` (`self.Plants`)) 3)
    (`self.Add_Plant` "/Game/Blueprints/Dirtland/Plant/Tornado/BP_Corn.BP_Corn_C")
    (else
      (`self.Watering_Plant`))))

(fn `Is_surviving`
  (params (NewParam :type "/Game/Blueprints/Enum/E_Disaster Enum" :default "NewEnumerator0"))
  (returns (survive :type Boolean))
  (locals (Land_Resistance :type "Float (double-precision)"))
  (set `local.Land_Resistance` 0.0)
  (for _array_element (`self.Plants`)
    (bind _resistance (`/Game/Blueprints/Dirtland/Plant/BP_Plant.Get_Resistance` _array_element NewParam))
    (set `local.Land_Resistance` (+ _resistance (`local.Land_Resistance`))))
  (return (> (`local.Land_Resistance`) 1.0)))

(fn `Relocate_Plant`
  (params (newPlant :type Boolean))
  (returns (NewParam :type "Vector Structure"))
  (locals (ListPosition :type "Set of Vector Structure") (New_Plant :type Boolean))
  (bind _plants (`self.Plants`))
  (set `local.New_Plant` newPlant)
  (switch `int` (- (`KismetArrayLibrary.Array_Length` (`self.Plants`)) (not newPlant))
    (:`0`
      _)
    (:`1`
      (set `local.ListPosition` (`self.Two_Plants_Position`)))
    (:`2`
      (set `local.ListPosition` (`self.Three_Plants_Position`))))
  (for (_array_element _array_index) _plants
    ; Repositionning old Plant
    (`self.K2_SetActorLocation` _array_element (+ (`BlueprintSetLibrary.Set_GetItemByIndex` (`local.ListPosition`) _array_index) (`self.K2_GetActorLocation`)) false false))
  (if (`local.New_Plant`)
    ; Positionning new Plant
    (return (`BlueprintSetLibrary.Set_GetItemByIndex` (`local.ListPosition`) (`KismetArrayLibrary.Array_Length` _plants)))
    (else
      (return (0.0 0.0 0.0)))))

(fn `Set_Material`
  (params (`Step On` :type Boolean) (MaterialToUse :type "Material Object Reference"))
  (bind _visualizer (`self.Visualizer`))
  (if `Step On`
    (`PrimitiveComponent.SetMaterial` _visualizer 0 "/Game/Materials/Dirtland/DirtlandReachable.DirtlandReachable")
    (else
      (`PrimitiveComponent.SetMaterial` _visualizer 0 "/Game/Materials/DirlandNotReachable.DirlandNotReachable")))
  (return))

(fn `Start_Selected`
  (params (caller :type "/Game/ThirdPerson/Blueprints/BP_ThirdPersonCharacter Object Reference"))
  (bind _asbp_farmer (cast `/Game/Blueprints/Farmer/BP_Farmer` caller)
    (:`then`
      (`PrimitiveComponent.SetMaterial` (`self.Visualizer`) 0 (`/Game/Blueprints/Farmer/BP_Farmer.Outline` _asbp_farmer))
      (set `self.IsFarmerOnIt` true))
    (:`CastFailed`
      (if (not (`self.IsFarmerOnIt`))
        (bind _asbp_phantom (cast `/Game/Blueprints/Phantom/BP_Phantom` caller))
        (`PrimitiveComponent.SetMaterial` (`self.Visualizer`) 0 (`/Game/Blueprints/Phantom/BP_Phantom.Outline` _asbp_phantom))))))

(fn `Stop_Selected`
  (params (Caller :type "/Game/ThirdPerson/Blueprints/BP_ThirdPersonCharacter Object Reference"))
  (cast `/Game/Blueprints/Farmer/BP_Farmer` Caller
    (:`then`
      (`PrimitiveComponent.SetMaterial` (`self.Visualizer`) 0 (`self.DefaultMaterial`))
      (set `self.IsFarmerOnIt` false))
    (:`CastFailed`
      (if (not (`self.IsFarmerOnIt`))
        (cast `/Game/Blueprints/Phantom/BP_Phantom` Caller)
        (`PrimitiveComponent.SetMaterial` (`self.Visualizer`) 0 (`self.DefaultMaterial`))))))

(fn `UserConstructionScript`)

(fn `Watering_Plant`
  (for _array_element (`self.Plants`)
    (bind _asbp_plant (cast `/Game/Blueprints/Dirtland/Plant/BP_Plant` _array_element))
    (if (`/Game/Blueprints/Dirtland/Plant/BP_Plant.Need_Water` _asbp_plant)
      (`/Game/Blueprints/Dirtland/Plant/BP_Plant.Watering` _array_element))))