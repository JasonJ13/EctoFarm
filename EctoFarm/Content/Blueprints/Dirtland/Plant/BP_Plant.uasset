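; BP_Plant is a farm plant that grows through phases, needing water between them, and is harvested via GI_EctoFarm.
; After a timed delay it shows a need widget; watering hides it, advances the phase and restarts the timer until the last phase.
; Phases are child components of Phases, swapped by visibility.
; It also looks up per-disaster resistance and can advance at night through NightReady, whose check is left unwired.
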(event `self.ReceiveBeginPlay`
  (`self.Display_Need` false)
  (`self.Grow`))

(event `Grow`
  (`KismetSystemLibrary.Delay` (`self.Timer_Phases`))
  (`self.Thirsty`))

(fn `Collect`
  (bind _asgi_ecto_farm (cast `/Game/Blueprints/GameInstance/GI_EctoFarm` (`GameplayStatics.GetGameInstance`)))
  (`/Game/Blueprints/GameInstance/GI_EctoFarm.Plant_Harvest` _asgi_ecto_farm self))

(fn `Display_Need`
  (params (Need :type Boolean))
  (`SceneComponent.SetHiddenInGame` (`self.Widget`) (not Need) true))

(fn `Get_Resistance`
  (params (Disaster :type "/Game/Blueprints/Enum/E_Disaster Enum" :default "NewEnumerator0"))
  (returns (Resistance :type "Float (double-precision)"))
  (bind (_value _returnvalue) (`BlueprintMapLibrary.Map_Find` (`self.Resistance`) Disaster))
  (if _returnvalue
    (return _value)
    (else
      (return 0.0))))

(fn `Next_Phase`
  ; Hide last Phase
  (`SceneComponent.SetVisibility` (`|GetArrayItem` (`SceneComponent.GetChildrenComponents` (`self.Phases`) false) (`self.ind_phase`)) false false)
  ; Set & Show New Phase
  (bind _output_get (set `self.ind_phase` (+ (`self.ind_phase`) 1)))
  (`SceneComponent.SetVisibility` (`|GetArrayItem` (`SceneComponent.GetChildrenComponents` (`self.Phases`) false) _output_get) true false)
  (return))

(fn `Night`
  (if (`self.Night_Ready`)
    (`self.Next_Phase`)))

(fn `Thirsty`
  (bind _output_get (set `self.Need_Water` true))
  (`self.Display_Need` _output_get))

(fn `UserConstructionScript`)

(fn `Watering`
  (bind _output_get (set `self.Need_Water` false))
  (`self.Display_Need` _output_get)
  (if (< (`self.ind_phase`) (- (`self.Nmb_Of_Phases`) 1))
    (`self.Next_Phase`)
    (`self.Grow`)
    (return)))