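; BP_Dirtland_Test_2 is a test Blueprint that checks survival on a Dirtland after planting two corn plants.
; On BeginPlay it runs the parent logic, calls AddPlant twice with BP_Corn, waits briefly, then prints the IsSurviving result for one enum value.
; AddPlant and IsSurviving are not defined in this file, and the overlap event is disabled.
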(event `self.ReceiveBeginPlay`
  (`parent.ReceiveBeginPlay`)
  (`self.Add_Plant` "/Game/BluePrints/Dirtland/Plant/BP_Corn.BP_Corn_C")
  (`self.Add_Plant` "/Game/BluePrints/Dirtland/Plant/BP_Corn.BP_Corn_C")
  (`KismetSystemLibrary.Delay` 5.0)
  (bind _survive (`self.Is_surviving` "NewEnumerator1"))
  (`KismetSystemLibrary.PrintString` (`KismetStringLibrary.Conv_BoolToString` _survive) true true (struct :`G` 1.0 :`B` 0.249509 :`A` 1.0) 5.0))

(fn `UserConstructionScript`
  (`parent.UserConstructionScript`))