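; BP_Phantom is a playable phantom that catches fairies and spends them on spells against the selected dirtland.
; Overlap events select the dirtland; three spells play a timed haunting, then erase one plant, all plants, or curse (placeholder).
; The haunting's affordability result is ignored, so effects still apply without enough fairies.
; Catching uses montage notifies to run looping right-arm overlap checks, updating the fairy count widget.
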(event `self.ReceiveBeginPlay`
  (`self.UI_Phantom_Setup`)
  (`self.WBP_init`))

(event `Haunting_Action`
  (params (malediction :type Integer))
  (bind _dirtlandselected (`self.DirtlandSelected`))
  (if (`self.OnDirtland`)
    (switch `int` malediction
      (:`0`
        (`self.Haunting` 5.0 3)
        (`KismetSystemLibrary.Delay` 5.0)
        (`self.Apply_Deplant` _dirtlandselected))
      (:`1`
        (`self.Haunting` 5.0 10)
        (`KismetSystemLibrary.Delay` 5.0)
        (`self.Apply_DeplantAll` _dirtlandselected))
      (:`2`
        (`self.Haunting` 5.0 10)
        (`KismetSystemLibrary.Delay` 5.0)
        (`self.Apply_Curse` _dirtlandselected)))
    (`self.End_Haunting`)
    (`/Game/UI/WBP_Phantom.Update_Fairy` (`self.WBP`) (`self.Nmb_Fairy`))))

(event `Player2_IA_Spell1`
  ; Phantom Actions on Dirtland (Spells)
  (`self.Haunting_Action` 0 :!label _label))

(event `self.ReceiveActorBeginOverlap`
  (params (OtherActor :type "Actor Object Reference"))
  ; When walking on a Dirtland, select it (and deselect previous one).
  (bind _asbp_dirtland (cast `/Game/Blueprints/Dirtland/BP_Dirtland` OtherActor))
  (if (`self.OnDirtland`)
    (`/Game/Blueprints/Dirtland/BP_Dirtland.Stop_Selected` (`self.DirtlandSelected`) self))
  (bind _output_get (set `self.DirtlandSelected` _asbp_dirtland))
  (set `self.OnDirtland` true)
  (`/Game/Blueprints/Dirtland/BP_Dirtland.Start_Selected` _output_get self))

(event `EnhancedInput|/Game/Input/Actions/Phantom/IA_PhantomSpell_1`
  (params (ActionValue :type Boolean) (ElapsedSeconds :type "Float (double-precision)") (TriggeredSeconds :type "Float (double-precision)") (InputAction :type "InputAction Object Reference" :default "/Game/Input/Actions/Phantom/IA_PhantomSpell_1.IA_PhantomSpell_1"))
  ; Phantom Actions on Dirtland (Spells)
  (:`Triggered`
    (goto _label)))

(event `Player2_IA_Spell2`
  ; Phantom Actions on Dirtland (Spells)
  (`self.Haunting_Action` 1 :!label _label_2))

(event `EnhancedInput|/Game/Input/Actions/Phantom/IA_PhantomSpell_2`
  (params (ActionValue :type Boolean) (ElapsedSeconds :type "Float (double-precision)") (TriggeredSeconds :type "Float (double-precision)") (InputAction :type "InputAction Object Reference" :default "/Game/Input/Actions/Phantom/IA_PhantomSpell_2.IA_PhantomSpell_2"))
  ; Phantom Actions on Dirtland (Spells)
  (:`Triggered`
    (goto _label_2)))

(event `self.ReceiveActorEndOverlap`
  (params (OtherActor :type "Actor Object Reference"))
  ; When walking out of a dirtland, deselect it.
  (bind _asbp_dirtland (cast `/Game/Blueprints/Dirtland/BP_Dirtland` OtherActor))
  (if (== _asbp_dirtland (`self.DirtlandSelected`))
    (`/Game/Blueprints/Dirtland/BP_Dirtland.Stop_Selected` (`self.DirtlandSelected`) self)
    (set `self.DirtlandSelected` null)
    (set `self.OnDirtland` false)))

(event `Player2_IA_Spell3`
  ; Phantom Actions on Dirtland (Spells)
  (`self.Haunting_Action` 2 :!label _label_3))

(event `EnhancedInput|/Game/Input/Actions/Phantom/IA_PhantomSpell_3`
  (params (ActionValue :type Boolean) (ElapsedSeconds :type "Float (double-precision)") (TriggeredSeconds :type "Float (double-precision)") (InputAction :type "InputAction Object Reference" :default "/Game/Input/Actions/Phantom/IA_PhantomSpell_3.IA_PhantomSpell_3"))
  ; Phantom Actions on Dirtland (Spells)
  (:`Triggered`
    (goto _label_3)))

(event `WBP_init`
  (bind _returnvalue (`|CreateWidget` "/Game/UI/WBP_Phantom.WBP_Phantom_C"))
  (bind _output_get (set `self.WBP` _returnvalue))
  (`UserWidget.AddToViewport` _output_get 0)
  (`KismetSystemLibrary.Delay` 2.0)
  (`/Game/UI/WBP_Phantom.Init` _output_get 2))

(event `Player2_IA_CatchFairy`
  ; Catch fairy
  (`/Engine/EditorBlueprintResources/StandardMacros.DoOnce` false :!label _label_4
    (:`Completed`
      (`self.DisableInput` (`self.AssignedPlayerController`))
      (`|PlayMontage` (`self.Mesh`) "/Game/Assets/Phantom/AM_Phantom_Catch.AM_Phantom_Catch"
        (:`OnNotifyBegin`
          (bind _returnvalue (`KismetSystemLibrary.K2_SetTimerDelegate` (delegate `Catch_Detection`) 0.1 true)))
        (:`OnNotifyEnd`
          (`self.Reset_Catch`)
          (`self.EnableInput` (`self.AssignedPlayerController`))
          (`KismetSystemLibrary.K2_ClearAndInvalidateTimerHandle` _returnvalue))))))

(event `EnhancedInput|/Game/Input/Actions/Phantom/IA_CatchFairy`
  (params (ActionValue :type Boolean) (ElapsedSeconds :type "Float (double-precision)") (TriggeredSeconds :type "Float (double-precision)") (InputAction :type "InputAction Object Reference" :default "/Game/Input/Actions/Phantom/IA_CatchFairy.IA_CatchFairy"))
  ; Catch fairy
  (:`Triggered`
    (goto _label_4)))

(event `Reset_Catch`
  ; Catch fairy
  (goto _label_4 :!via `Reset`))

(event `Catch_Detection`
  ; Catch fairy
  (for _array_element (`PrimitiveComponent.GetOverlappingActors` (`self.Right_Arm`) "/Game/Blueprints/Fairy/BP_Fairy.BP_Fairy_C")
    (`self.CatchFairy` _array_element)))

(fn `Apply_Curse`
  (params (Dirtland_To_Curse :type "/Game/Blueprints/Dirtland/BP_Dirtland Object Reference"))
  (`KismetSystemLibrary.PrintText` "TBA  (Curse)"))

(fn `Apply_Deplant`
  (params (Dirtland_To_Deplant :type "/Game/Blueprints/Dirtland/BP_Dirtland Object Reference"))
  (`/Game/Blueprints/Dirtland/BP_Dirtland.Erase_One_Plant` Dirtland_To_Deplant))

(fn `Apply_DeplantAll`
  (params (Dirtland_To_DeplantAll :type "/Game/Blueprints/Dirtland/BP_Dirtland Object Reference"))
  (`/Game/Blueprints/Dirtland/BP_Dirtland.Erase_All_Plant` Dirtland_To_DeplantAll))

(fn `CatchFairy`
  (params (Fairy :type "Actor Object Reference"))
  (`self.K2_DestroyActor` Fairy)
  (bind _output_get (set `self.Nmb_Fairy` (+ (`self.Nmb_Fairy`) 1)))
  (`/Game/UI/WBP_Phantom.Update_Fairy` (`self.WBP`) _output_get))

(fn `End_Haunting`
  (`SceneComponent.SetVisibility` (`self.Widget_UI`) false true)
  (`self.StopAnimMontage` "/Game/Assets/Phantom/AM_Phantom_Haunting.AM_Phantom_Haunting"))

(fn `Haunting`
  (params (Haunting_Duration :type "Float (double-precision)") (Cost :type Integer))
  (returns (Haunt :type Boolean))
  (locals (duration :type "Float (double-precision)"))
  (if (> (`self.Nmb_Fairy`) Cost)
    (set `self.Nmb_Fairy` (- (`self.Nmb_Fairy`) Cost))
    (set `local.duration` Haunting_Duration)
    (`self.PlayAnimMontage` "/Game/Assets/Phantom/AM_Phantom_Haunting.AM_Phantom_Haunting")
    (`SceneComponent.SetVisibility` (`self.Widget_UI`) true true)
    (bind _asui_phantom (cast `/Game/Blueprints/Phantom/UI_Phantom` (`WidgetComponent.GetWidget` (`self.Widget_UI`))))
    (`/Game/Blueprints/Phantom/UI_Phantom.New_Haunting` _asui_phantom (`local.duration`))
    (return true)
    (else
      (return false))))

(fn `NewFunction`)

(fn `Pushed`
  (`self.AddMovementInput` (0.0 0.0 0.0)))

(fn `UI_Phantom_Setup`
  (bind _asui_phantom (cast `/Game/Blueprints/Phantom/UI_Phantom` (`WidgetComponent.GetWidget` (`self.Widget_UI`))))
  (set `/Game/Blueprints/Phantom/UI_Phantom.BP_Owner` self _asui_phantom))

(fn `UserConstructionScript`
  (`parent.UserConstructionScript`))