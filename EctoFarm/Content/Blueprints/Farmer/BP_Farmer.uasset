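; BP_Farmer is the farmer player, who plants, waters and harvests dirt plots and bumps the Phantom player.
; Overlap selects the current BP_Dirtland for actions, while three rotating seed slots feed planting and the HUD widget.
; A montage notify window runs a looping timer that checks head overlaps for bump hits.
; Menu input, routed by state flags, drives the tutorial, GameMode seed purchases and the night widget's loadout selection.
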(event `tutorial`
  (`/Game/UI/WBP_Farmer.Next_tutorial` (`self.WBP`))
  (`EnhancedInputSubsystemInterface.AddMappingContext` (subsystem `EnhancedInputLocalPlayerSubsystem`) "/Game/Input/IMC_Menu.IMC_Menu" 0 (struct))
  (set `self.In_Tutorial` true)
  (`KismetSystemLibrary.PrintString` "active tuto"))

(event `EnhancedInput|/Game/Input/Actions/Menu/IA_Move_Shop`
  (params (ActionValue :type "Vector2D Structure") (ElapsedSeconds :type "Float (double-precision)") (TriggeredSeconds :type "Float (double-precision)") (InputAction :type "InputAction Object Reference" :default "/Game/Input/Actions/Menu/IA_Move_Shop.IA_Move_Shop"))
  ; Shopping phase
  ;; Moving in shot
  (:`Triggered`
    (`self.Move_In_Menu` ActionValue)))

(event `EnhancedInput|/Game/Input/Actions/Menu/IA_Menu_Confirm`
  (params (ActionValue :type Boolean) (ElapsedSeconds :type "Float (double-precision)") (TriggeredSeconds :type "Float (double-precision)") (InputAction :type "InputAction Object Reference" :default "/Game/Input/Actions/Menu/IA_Menu_Confirm.IA_Menu_Confirm"))
  ; Shopping phase
  ;; Buying in shop
  (:`Triggered`
    (`self.Act_in_Menu` (`self.Position_Shop`))))

(event `self.ReceiveBeginPlay`
  (`self.WBP_init`)
  (`/Game/UI/WBP_Farmer.Change_Name` (`self.WBP`) (`self.Seed1`) (`self.Seed2`) (`self.Seed3`)))

(event `EnhancedInput|/Game/Input/Actions/Farmer/IA_Plant`
  (params (ActionValue :type Boolean) (ElapsedSeconds :type "Float (double-precision)") (TriggeredSeconds :type "Float (double-precision)") (InputAction :type "InputAction Object Reference" :default "/Game/Input/Actions/Farmer/IA_Plant.IA_Plant"))
  ; Basic Action on DirtLand
  (:`Triggered`
    (if (`self.OnDirtland`)
      (bind (_seed_to_plant _wascanceled) (`self.Select_Seed`))
      (if (not _wascanceled)
        (`/Game/Blueprints/Dirtland/BP_Dirtland.Add_Plant` (`self.DirtlandSelected`) _seed_to_plant)))))

(event `EnhancedInput|/Game/Input/Actions/Farmer/IA_Water`
  (params (ActionValue :type Boolean) (ElapsedSeconds :type "Float (double-precision)") (TriggeredSeconds :type "Float (double-precision)") (InputAction :type "InputAction Object Reference" :default "/Game/Input/Actions/Farmer/IA_Water.IA_Water"))
  ; Basic Action on DirtLand
  (:`Triggered`
    (if (`self.OnDirtland`)
      (`/Game/Blueprints/Dirtland/BP_Dirtland.Watering_Plant` (`self.DirtlandSelected`)))))

(event `self.ReceiveActorBeginOverlap`
  (params (OtherActor :type "Actor Object Reference"))
  ; When walking on a Dirtland, select it (and deselect previous one).
  (bind _asbp_dirtland (cast `/Game/Blueprints/Dirtland/BP_Dirtland` OtherActor))
  (if (`self.OnDirtland`)
    (`/Game/Blueprints/Dirtland/BP_Dirtland.Stop_Selected` (`self.DirtlandSelected`) self))
  (bind _output_get (set `self.DirtlandSelected` _asbp_dirtland))
  (set `self.OnDirtland` true)
  (`/Game/Blueprints/Dirtland/BP_Dirtland.Start_Selected` _output_get self))

(event `EnhancedInput|/Game/Input/Actions/Farmer/IA_Harvest`
  (params (ActionValue :type Boolean) (ElapsedSeconds :type "Float (double-precision)") (TriggeredSeconds :type "Float (double-precision)") (InputAction :type "InputAction Object Reference" :default "/Game/Input/Actions/Farmer/IA_Harvest.IA_Harvest"))
  ; Basic Action on DirtLand
  (:`Triggered`
    (if (`self.OnDirtland`)
      (`/Game/Blueprints/Dirtland/BP_Dirtland.Harvest` (`self.DirtlandSelected`)))))

(event `EnhancedInput|/Game/Input/Actions/Farmer/IA_Seed_Next`
  (params (ActionValue :type Boolean) (ElapsedSeconds :type "Float (double-precision)") (TriggeredSeconds :type "Float (double-precision)") (InputAction :type "InputAction Object Reference" :default "/Game/Input/Actions/Farmer/IA_Seed_Next.IA_Seed_Next"))
  ; Change Seed
  (:`Triggered`
    (`self.Next_Seed` true)))

(event `self.ReceiveActorEndOverlap`
  (params (OtherActor :type "Actor Object Reference"))
  ; When walking out of a dirtland, deselect it.
  (bind _asbp_dirtland (cast `/Game/Blueprints/Dirtland/BP_Dirtland` OtherActor))
  (if (== _asbp_dirtland (`self.DirtlandSelected`))
    (`/Game/Blueprints/Dirtland/BP_Dirtland.Stop_Selected` (`self.DirtlandSelected`) self)
    (set `self.DirtlandSelected` null)
    (set `self.OnDirtland` false)))

(event `EnhancedInput|/Game/Input/Actions/Farmer/IA_Seed_past`
  (params (ActionValue :type Boolean) (ElapsedSeconds :type "Float (double-precision)") (TriggeredSeconds :type "Float (double-precision)") (InputAction :type "InputAction Object Reference" :default "/Game/Input/Actions/Farmer/IA_Seed_past.IA_Seed_past"))
  ; Change Seed
  (:`Triggered`
    (`self.Next_Seed` false)))

(event `WBP_init`
  (bind _returnvalue (`|CreateWidget` "/Game/UI/WBP_Farmer.WBP_Farmer_C"))
  (bind _output_get (set `self.WBP` _returnvalue))
  (`UserWidget.AddToViewport` _output_get 0))

(event `EnhancedInput|/Game/Input/Actions/Farmer/IA_Bump`
  (params (ActionValue :type Boolean) (ElapsedSeconds :type "Float (double-precision)") (TriggeredSeconds :type "Float (double-precision)") (InputAction :type "InputAction Object Reference" :default "/Game/Input/Actions/Farmer/IA_Bump.IA_Bump"))
  ; Catch fairy
  (:`Triggered`
    (`/Engine/EditorBlueprintResources/StandardMacros.DoOnce` false :!label _label
      (:`Completed`
        (`self.DisableInput` (`self.AssignedPlayerController`))
        (`|PlayMontage` (`self.Mesh`) "/Game/Assets/Farmer/AM_Farmer_bump.AM_Farmer_bump"
          (:`OnCompleted`
            (`self.Reset_Bump` :!label _label_2)
            (`self.EnableInput` (`self.AssignedPlayerController`))
            (`KismetSystemLibrary.K2_ClearAndInvalidateTimerHandle` (stale _returnvalue)))
          (:`OnInterrupted`
            (goto _label_2))
          (:`OnNotifyBegin`
            (bind _returnvalue (`KismetSystemLibrary.K2_SetTimerDelegate` (delegate `Bump_Detection`) 0.1 true)))
          (:`OnNotifyEnd`
            (goto _label_2)))))))

(event `Reset_Bump`
  ; Catch fairy
  (goto _label :!via `Reset`))

(event `Bump_Detection`
  ; Catch fairy
  (for _array_element (`PrimitiveComponent.GetOverlappingActors` (`self.Head_0`) "/Game/Blueprints/Phantom/BP_Phantom.BP_Phantom_C")
    (bind _asbp_phantom (cast `/Game/Blueprints/Phantom/BP_Phantom` _array_element))
    (`/Game/Blueprints/Phantom/BP_Phantom.bumped` _asbp_phantom)))

(fn `Act_in_Menu`
  (params (Position :type Integer))
  (locals (Seed_Bought :type "/Game/Blueprints/Dirtland/Plant/BP_Plant Class Reference") (New_Found :type Integer))
  (bind _seed_select (`self.Seed_Select`))
  (bind _wbp_night (`self.WBP_Night`))
  (if (`self.In_Tutorial`)
    (`KismetSystemLibrary.PrintString` "next")
    (bind _end (`/Game/UI/WBP_Farmer.Next_tutorial` (`self.WBP`)))
    (if _end
      (`self.End_Tutorial`))
    (elif (`self.In_Shop`)
      (bind _asgm_multi (cast `/Game/Gamemode/GM_Multi` (`GameplayStatics.GetGameMode`)))
      (bind (_as_bought _seed_bought) (`/Game/Gamemode/GM_Multi.Buy_Seed` _asgm_multi Position))
      (`KismetSystemLibrary.PrintString` (`KismetStringLibrary.Conv_BoolToString` _as_bought))
      (if _as_bought
        (`KismetArrayLibrary.Array_Add` (`self.BoughtSeeds`) _seed_bought))
      (else
        (`/Game/UI/Night/WBP_Night.Switch_Selection` (`self.WBP_Night`) false)
        (if (`self.In_Selection_1`)
          (`/Game/UI/Night/WBP_Night.Switch_Selection` (`self.WBP_Night`) (`self.In_Selection_1`))
          (set `self.In_Selection_1` false)
          (bind _output_get (set `self.Position_Inventory` 1))
          (`/Game/UI/Night/WBP_Night.Move_Inventory` _wbp_night _output_get)
          (else
            (set `self.In_Selection_1` true)
            (switch `int` (`self.Position_Inventory`)
              (:`0`
                (set `self.Seed1` _seed_select))
              (:`1`
                (set `self.Seed2` _seed_select))
              (:`2`
                (set `self.Seed3` _seed_select)))
            (`/Game/UI/Night/WBP_Night.Replace_Seed` _wbp_night (`self.Position_Inventory`) _seed_select)
            (`/Game/UI/Night/WBP_Night.Switch_Selection` (`self.WBP_Night`) (`self.In_Selection_1`))
            (set `self.In_Selection_1` true)))))))

(fn `Begin_Shop`
  (params (WBP :type "/Game/UI/Night/WBP_Night Object Reference"))
  (set `self.WBP_Night` WBP)
  (set `self.Position_Shop` 0)
  (`EnhancedInputSubsystemInterface.AddMappingContext` (subsystem `EnhancedInputLocalPlayerSubsystem`) "/Game/Input/IMC_Menu.IMC_Menu" 0 (struct))
  (set `self.In_Shop` true))

(fn `Day_Time`
  (`/Game/UI/WBP_Farmer.Change_Name` (`self.WBP`) (`self.Seed1`) (`self.Seed2`) (`self.Seed2`)))

(fn `End_Shop`
  (set `self.In_Shop` false))

(fn `End_Tutorial`)

(fn `initializePlayer2`
  (bind _outactors (`GameplayStatics.GetAllActorsOfClass` "/Game/Blueprints/Phantom/BP_Phantom.BP_Phantom_C"))
  (set `self.Player2` (`|GetArrayItem` _outactors)))

(fn `Move_In_Menu`
  (params (mouvement :type "Vector2D Structure"))
  (locals (New_Position :type Integer) (mouv :type "Vector2D Structure"))
  (if (`self.In_Tutorial`)
    (return)
    (else
      (set `local.mouv` mouvement)
      (if (`self.In_Shop`)
        (bind _output_get (set `self.Position_Shop` (`self.Macro_Position` (`local.mouv`) (`self.Position_Shop`))))
        (`/Game/UI/Night/WBP_Night.Move_Shop` (`self.WBP_Night`) _output_get)
        (elif (`self.In_Selection_1`)
          (bind _ind (`/Game/UI/Night/WBP_Night.Move_Selection` (`self.WBP_Night`) (`local.mouv`)))
          (set `self.Seed_Select` (`|GetArrayItem` (`self.BoughtSeeds`) _ind))
          (else
            (bind _output_get_2 (set `self.Position_Inventory` (`self.Macro_Position` (`local.mouv`) (`self.Position_Inventory`))))
            (`/Game/UI/Night/WBP_Night.Move_Inventory` (`self.WBP_Night`) _output_get_2)))))))

(fn `Next_Seed`
  (params (forward :type Boolean))
  (locals (Temp_Seed :type "/Game/Blueprints/Dirtland/Plant/BP_Plant Class Reference"))
  (set `local.Temp_Seed` (`self.Seed1`))
  (if forward
    (set `self.Seed1` (`self.Seed2`))
    (set `self.Seed2` (`self.Seed3`))
    (bind _output_get (set `self.Seed3` (`local.Temp_Seed`)))
    (else
      (set `self.Seed1` (`self.Seed3`))
      (set `self.Seed3` (`self.Seed2`))
      (bind _output_get_2 (set `self.Seed2` (`local.Temp_Seed`)))))
  (`/Game/UI/WBP_Farmer.Change_Name` (`self.WBP`) (`self.Seed1`) _output_get_2 _output_get))

(fn `Night_Time`
  (`EnhancedInputSubsystemInterface.RemoveMappingContext` (subsystem `EnhancedInputLocalPlayerSubsystem`) "/Game/Input/IMC_Default.IMC_Default" (struct)))

(fn `Seed_Selection`
  (params (duration :type "Float (double-precision)"))
  (`/Game/UI/Night/WBP_Night.Seeds_Selection_Phase` (`self.WBP_Night`) (`self.BoughtSeeds`) (`|MakeArray` (`self.Seed1`) (`self.Seed2`) (`self.Seed3`)) duration))

(fn `Select_Seed`
  (returns (Seed_To_Plant :type "/Game/Blueprints/Dirtland/Plant/BP_Plant Class Reference") (WasCanceled :type Boolean))
  (return (`self.Seed1`) false))

(fn `UserConstructionScript`
  (`parent.UserConstructionScript`))