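; BP_Fairy_Spawner_Tool is a fairy spawner driven by an on-screen tool widget.
; On BeginPlay it runs the parent logic, creates WBP_Fairy_tool, binds the widget's fairy spawn event to FairySpawn, and adds it to the viewport.
; A separate custom event calls AddFairy with a negative one, but nothing in this graph binds or calls it.
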(event `self.ReceiveBeginPlay`
  (`parent.ReceiveBeginPlay`)
  (bind _returnvalue (`|CreateWidget` "/Game/BluePrints/Fairy/WBP_Fairy_tool.WBP_Fairy_tool_C"))
  (bind _output_get (set `self.WBP` _returnvalue))
  (add `/Game/BluePrints/Fairy/WBP_Fairy_tool.FairySpawn` _returnvalue (delegate `CustomEvent`))
  (add `/Game/BluePrints/Fairy/WBP_Fairy_tool.FairySpawn` _output_get (delegate `CustomEvent`))
  (`UserWidget.AddToViewport` _returnvalue 0))

(event `CustomEvent`
  (`self.Fairy_spawn`))

(event `CustomEvent_1`
  (`self.Add_Fairy` -1))

(fn `UserConstructionScript`
  (`parent.UserConstructionScript`))