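; BP_Plant is a plant actor with phase meshes and a widget that signals when it needs water.
; On BeginPlay it disables collision on the static meshes under Phases and hides the water widget.
; NeedWater toggles that widget, while NewPhase hides the child mesh at the current phase index and increments it, without explicitly showing the next.
; A delayed NeedWater test is left unconnected.
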(event `self.ReceiveBeginPlay`
  (for _array_element (`SceneComponent.GetChildrenComponents` (`self.Phases`) false)
    (bind _asstatic_mesh_component (cast `StaticMeshComponent` _array_element))
    (`PrimitiveComponent.SetCollisionEnabled` _asstatic_mesh_component "NoCollision"))
  (`self.Need_Water` false))

(fn `Need_Water`
  (params (Need :type Boolean))
  (`SceneComponent.SetHiddenInGame` (`self.Widget`) (not Need) true))

(fn `New_Phase`
  (`SceneComponent.SetVisibility` (`|GetArrayItem` (`SceneComponent.GetChildrenComponents` (`self.Phases`) false) (`self.ind_phase`)) false false)
  (set `self.ind_phase` (+ (`self.ind_phase`) 1))
  (return))

(fn `UserConstructionScript`)