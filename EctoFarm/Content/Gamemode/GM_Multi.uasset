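; Game mode for local multiplayer that spawns a team of Farmers and a team of Phantoms.
; On BeginPlay it creates the extra Farmer players, switches the default pawn class to BP_Phantom, creates the remaining players, then prints connected input devices.
; Each created character stores its controller and player ID.
; ChoosePlayerStart uses the current default pawn class to pick the first PlayerStart found for Farmers, the second otherwise.
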(event `self.ReceiveBeginPlay`
  (bind _numberoffarmer (`self.NumberOfFarmer`))
  ; Spawning Farmers and Phantoms
  (for _index (range 1 _numberoffarmer)
    (bind _returnvalue (`GameplayStatics.CreatePlayer` _index))
    (bind _asbp_third_person_character (cast `/Game/ThirdPerson/Blueprints/BP_ThirdPersonCharacter` (`Controller.K2_GetPawn` _returnvalue)))
    (bind _output_get (set `/Game/ThirdPerson/Blueprints/BP_ThirdPersonCharacter.AssignedPlayerController` _returnvalue _asbp_third_person_character))
    (set `/Game/ThirdPerson/Blueprints/BP_ThirdPersonCharacter.Player_ID` (`GameplayStatics.GetPlayerControllerID` _output_get) _asbp_third_person_character))
  (set `self.DefaultPawnClass` "/Game/Blueprints/Phantom/BP_Phantom.BP_Phantom_C")
  (for _index_2 (range _numberoffarmer (+ (`self.NumberOfPlayers`) 1))
    (bind _returnvalue_2 (`GameplayStatics.CreatePlayer` _index_2))
    (bind _asbp_third_person_character_2 (cast `/Game/ThirdPerson/Blueprints/BP_ThirdPersonCharacter` (`Controller.K2_GetPawn` _returnvalue_2)))
    (bind _output_get_2 (set `/Game/ThirdPerson/Blueprints/BP_ThirdPersonCharacter.AssignedPlayerController` _returnvalue_2 _asbp_third_person_character_2))
    (set `/Game/ThirdPerson/Blueprints/BP_ThirdPersonCharacter.Player_ID` (`GameplayStatics.GetPlayerControllerID` _output_get_2) _asbp_third_person_character_2))
  (bind _outinputdevices (`InputDeviceLibrary.GetAllConnectedInputDevices`))
  (for _array_element _outinputdevices
    (`KismetSystemLibrary.PrintString` (`KismetStringLibrary.Conv_InputDeviceIdToString` _array_element))))

(fn `ChoosePlayerStart`
  (params (Player :type "Controller Object Reference"))
  (returns (ReturnValue :type "Actor Object Reference"))
  (locals (NewLocalVar :type Boolean) (StartNumber :type Integer))
  (bind _outactors (`GameplayStatics.GetAllActorsOfClass` "/Script/Engine.PlayerStart"))
  (if (== (`self.DefaultPawnClass`) "/Game/Blueprints/Farmer/BP_Farmer.BP_Farmer_C")
    (set `local.StartNumber` 0)
    (bind _output (`|GetArrayItem` _outactors (stale _output_get)))
    (return _output)
    (else
      (bind _output_get (set `local.StartNumber` 1))
      (return _output))))

(fn `UserConstructionScript`)